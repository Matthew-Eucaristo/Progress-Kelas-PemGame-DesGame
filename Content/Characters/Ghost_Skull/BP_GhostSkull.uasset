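; BP_GhostSkull is a flying skull enemy that patrols, then chases and shoots at the player.
; While idle it moves to random BP_PatrolLocation actors; PawnSensing sightings start a chase, and a periodic distance check toggles IDLE/CHASING and the looping animation.
; Tick drives turning toward a nearby player, state checks, bullet spawning while chasing, and unclamped self-healing, using Delays as throttles.
; The patrol loop ends outside IDLE and is never restarted.
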(event OnSeePawn(PawnSensing)
  (params (Pawn :type Pawn%20Object%20Reference))
  (Utilities|FlowControl|Sequence
    (:then_0
      (AI|AIMoveTo self "0, 0, 0" Pawn 1e+02 false))
    (:then_1
      (Variables|Default|SetSTATE "NewEnumerator1"))))

(event Custom|Rotate%20to%20face%20the%20player
  (if (CallFunction|IsNearEnough)
    (Transformation|SetWorldRotation (Variables|Default|GetCapsuleComponent) (Math|Rotator|Lerp(Rotator) (Transformation|GetWorldRotation (Variables|Default|GetCapsuleComponent)) (Math|Rotator|FindLookatRotation (Transformation|GetWorldLocation (Variables|Default|GetCapsuleComponent)) (Transformation|GetWorldLocation (Variables|/Script/Engine.Character|GetCapsuleComponent (Game|GetPlayerCharacter 0)))) 0.5 true) false false)))

(event Custom|Cycle%20Animation
  (switch Utilities|FlowControl|Switch|SwitchonENUM_GhostState (Variables|Default|GetSTATE)
    (:NewEnumerator0
      (Components|Animation|PlayAnimation (Variables|Character|GetMesh) "/Game/Characters/Ghost_Skull/Ghost_Skull_Anim_CharacterArmature_Flying_Idle.Ghost_Skull_Anim_CharacterArmature_Flying_Idle" true))
    (:NewEnumerator1
      (Components|Animation|PlayAnimation (Variables|Character|GetMesh) "/Game/Characters/Ghost_Skull/Ghost_Skull_Anim_CharacterArmature_Fast_Flying.Ghost_Skull_Anim_CharacterArmature_Fast_Flying" true))))

(event Custom|Check%20State%20Periodically
  (Utilities|FlowControl|Delay 2.0)
  (if (CallFunction|IsNearEnough)
    (Variables|Default|SetSTATE "NewEnumerator1")
    (else
      (Variables|Default|SetSTATE "NewEnumerator0")))
  (CallFunction|CycleAnimation))

(event Custom|Shoot
  (Utilities|FlowControl|Delay 0.7)
  (switch Utilities|FlowControl|Switch|SwitchonENUM_GhostState (Variables|Default|GetSTATE)
    (:NewEnumerator1
      (Game|SpawnActorfromClass "/Game/Characters/Ghost_Skull/Weapon/Bullet/BP_AKBullets.BP_AKBullets_C" (Transformation|GetWorldTransform (Variables|Default|GetBulletOut)) "AlwaysSpawn" "MultiplyWithRoot" 0 0))))

(event Custom|Patrol%20to%20Location
  (switch Utilities|FlowControl|Switch|SwitchonENUM_GhostState (Variables|Default|GetSTATE)
    (:NewEnumerator0
      (bind _outactors (Actor|GetAllActorsOfClass "/Game/BP_PatrolLocation.BP_PatrolLocation_C"))
      (bind _output_get (Variables|Default|SetPatrol%20Location _outactors))
      (AI|AIMoveTo self "0, 0, 0" (.OutItem (Utilities|Array|Random _output_get)) 5.0 false
        (:then
          (Utilities|FlowControl|Delay 2.0)
          (CallFunction|PatroltoLocation))))))

(event Custom|Self%20Heal
  (Utilities|FlowControl|Delay 2.0)
  (Variables|Default|SetHealth (+ (Variables|Default|GetHealth) (* (Variables|Default|GetMax%20Health) 0.1))))

(event EventBeginPlay
  (CallFunction|PatroltoLocation)
  (Variables|Default|SetName "Mikey")
  (Variables|Default|SetHealth 2e+02))

(event Collision|EventActorBeginOverlap
  (params (OtherActor :type Actor%20Object%20Reference)))

(event EventTick
  (params (DeltaSeconds :type Float%20%28single-precision%29))
  (CallFunction|RotatetoFacethePlayer)
  (CallFunction|CheckStatePeriodically)
  (CallFunction|Shoot)
  (CallFunction|SelfHeal))

(fn ConstructionScript)

(fn IsNearEnough
  (return (< (Math|Vector|Distance(Vector) (Transformation|GetWorldLocation (Variables|/Script/Engine.Character|GetCapsuleComponent (Game|GetPlayerCharacter 0))) (Transformation|GetWorldLocation (Variables|Default|GetCapsuleComponent))) (Variables|Default|GetDistance%20to%20notice))))